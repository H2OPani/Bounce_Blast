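; BP_Enemy is an enemy that chases the player, fires bullets and damages the player on contact.
; Once the third-person character enters SenseRange, it moves via AIMoveTo on Tick, yaws toward the player and starts a looping timer spawning four BP_Bullets at fixed, non-aimed rotations.
; Hit lowers Health, updates the health widget and destroys the enemy at zero.
; Capsule overlap with the sensed player deals damage and destroys the enemy.
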(event `self.ReceiveBeginPlay`
  (bind _aswbp_enemy_health (cast `/Game/Widgets/WBP_EnemyHealth` (`WidgetComponent.GetWidget` (`self.Widget`))))
  (set `self.WBP_EnemyHealtth` _aswbp_enemy_health))

(event `self.ReceiveTick`
  (params (DeltaSeconds :type "Float (single-precision)"))
  (bind (_returnvalue_roll _returnvalue_pitch _returnvalue_yaw) (`KismetMathLibrary.BreakRotator` (`KismetMathLibrary.FindLookAtRotation` (`self.K2_GetActorLocation`) (`self.K2_GetActorLocation` (`GameplayStatics.GetPlayerPawn` 0)))))
  (if (`self.CanSee?`)
    (`|AIMoveTo` self (0.0 0.0 0.0) (stale `self.SenseRange.OnComponentBeginOverlap` OtherActor) 3.0
      (:`then`
        (`self.K2_SetActorRotation` (`KismetMathLibrary.MakeRotator` 0.0 0.0 _returnvalue_yaw))))))

(event `/Game/blueprints/Interfaces/BPI_Hit.Hit`
  (params (Damage :type "Float (double-precision)"))
  (bind _output_get (set `self.Health` (- (`self.Health`) Damage)))
  (bind _output_get_2 (set `/Game/Widgets/WBP_EnemyHealth.GetHealth` _output_get (`self.WBP_EnemyHealtth`)))
  (if (<= _output_get_2 0.0)
    (`self.K2_DestroyActor`)))

(event `self.SenseRange.OnComponentBeginOverlap`
  (params (OverlappedComponent :type "PrimitiveComponent Object Reference") (OtherActor :type "Actor Object Reference") (OtherComp :type "PrimitiveComponent Object Reference") (OtherBodyIndex :type Integer) (bFromSweep :type Boolean) (SweepResult :type "HitResult Structure (by ref)"))
  (bind _asbp_third_person_character (cast `/Game/ThirdPerson/Blueprints/BP_ThirdPersonCharacter` OtherActor))
  (set `self.As BP Third Person Character` _asbp_third_person_character)
  (set `self.CanSee?` true)
  (`KismetSystemLibrary.K2_SetTimerDelegate` (delegate `Timer`) (`self.Time`) true))

(event `Timer`
  (bind _returnvalue (`self.K2_GetActorLocation`))
  (`GameplayStatics.PlaySound2D` "/Game/sound-work-futuristic-gun-shot-sci-fi-217154.sound-work-futuristic-gun-shot-sci-fi-217154" 2.5 1.0 0.0 null null)
  (`|SpawnActorFromClass` "/Game/blueprints/BP_Bullet.BP_Bullet_C" (`KismetMathLibrary.MakeTransform` _returnvalue) "Undefined" "MultiplyWithRoot" null null)
  (`|SpawnActorFromClass` "/Game/blueprints/BP_Bullet.BP_Bullet_C" (`KismetMathLibrary.MakeTransform` _returnvalue (struct :`Yaw` 90.0)) "Undefined" "MultiplyWithRoot" null null)
  (`|SpawnActorFromClass` "/Game/blueprints/BP_Bullet.BP_Bullet_C" (`KismetMathLibrary.MakeTransform` _returnvalue (struct :`Yaw` -90.0)) "Undefined" "MultiplyWithRoot" null null)
  (`|SpawnActorFromClass` "/Game/blueprints/BP_Bullet.BP_Bullet_C" (`KismetMathLibrary.MakeTransform` _returnvalue (struct :`Yaw` 45.0)) "Undefined" "MultiplyWithRoot" null null))

(event `self.Capsule.OnComponentBeginOverlap`
  (params (OverlappedComponent :type "PrimitiveComponent Object Reference") (OtherActor :type "Actor Object Reference") (OtherComp :type "PrimitiveComponent Object Reference") (OtherBodyIndex :type Integer) (bFromSweep :type Boolean) (SweepResult :type "HitResult Structure (by ref)"))
  (bind _as_bp_third_person_character (`self.As BP Third Person Character`))
  (if (== OtherActor _as_bp_third_person_character)
    (`/Game/blueprints/Interfaces/BPI_Hit.Hit` _as_bp_third_person_character (`self.Damage`))
    (`self.K2_DestroyActor`)))

(fn `UserConstructionScript`)