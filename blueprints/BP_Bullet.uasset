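; BP_Bullet is a bullet actor that deals damage to actors it overlaps.
; On BeginPlay it sets a just-spawned flag and disables mesh and capsule collision, then restores both after a short delay.
; Once that grace period ends, a capsule overlap passes Damage to the other actor through HitMessage.
; The graph contains no movement or destroy logic.
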(event `self.ReceiveBeginPlay`
  (set `self.DidJustSpawn` true)
  (`PrimitiveComponent.SetCollisionEnabled` (`self.StaticMesh`) "NoCollision")
  (`PrimitiveComponent.SetCollisionEnabled` (`self.Capsule`) "NoCollision")
  (`KismetSystemLibrary.Delay` 0.2)
  (set `self.DidJustSpawn` false)
  (`PrimitiveComponent.SetCollisionEnabled` (`self.StaticMesh`) "QueryAndPhysics")
  (`PrimitiveComponent.SetCollisionEnabled` (`self.Capsule`) "QueryAndPhysics"))

(event `self.Capsule.OnComponentBeginOverlap`
  (params (OverlappedComponent :type "PrimitiveComponent Object Reference") (OtherActor :type "Actor Object Reference") (OtherComp :type "PrimitiveComponent Object Reference") (OtherBodyIndex :type Integer) (bFromSweep :type Boolean) (SweepResult :type "HitResult Structure (by ref)"))
  (if (not (`self.DidJustSpawn`))
    (message `/Game/blueprints/Interfaces/BPI_Hit.Hit` OtherActor (`self.Damage`))))

(fn `UserConstructionScript`)